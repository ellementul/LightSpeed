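; Game instance blueprint that handles level flow between the main menu and game world, plus a persistent record table of player results.
; BeginGame, ExitToMainMenu and Quit control navigation, while GameOver records the player state's name, points and scaled distance before returning to the menu.
; LoadTable loads the RecordTable save slot or creates a new one, feeding AddRecord, which timestamps and saves entries, and GetRecordList, which returns them.
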(event `BeginGame`
  (`GameplayStatics.OpenLevel` "GameWorld"))

(event `GameOver`
  (params (PlayerController :type "/Game/Core/BP_PC Object Reference"))
  ;[1 1 1] GameOver
  (bind _asbp_ps (cast `/Game/Core/BP_PS` (`Controller.PlayerState` PlayerController)))
  (`self.AddRecord` (`/Game/Core/BP_PS.Name` _asbp_ps) (`/Game/Core/BP_PS.Points` _asbp_ps) (`KismetMathLibrary.FTrunc` (/ (`/Game/Core/BP_PS.Distance` _asbp_ps) 100.0)))
  (`self.ExitToMainMenu`))

(event `ExitToMainMenu`
  (`GameplayStatics.OpenLevel` "MainMenu"))

(event `Quit`
  (`KismetSystemLibrary.QuitGame` null "Quit"))

(fn `AddRecord`
  (params (PlayerName :type Text) (Points :type Integer) (Distance :type Integer))
  (bind _returntable (`self.LoadTable`))
  (`/Game/Core/RecordTable.AddRecord` _returntable (make `/Game/Core/Record` PlayerName Points Distance (`KismetMathLibrary.Now`)))
  (`GameplayStatics.SaveGameToSlot` _returntable (`self.RecordTableName`)))

(fn `GetRecordList`
  (returns (Table :type "Array of /Game/Core/Record Structure"))
  (bind _returntable (`self.LoadTable`))
  (return (`/Game/Core/RecordTable.Table` _returntable)))

(fn `LoadTable`
  (returns (ReturnTable :type "/Game/Core/RecordTable Object Reference"))
  (locals (Table :type "/Game/Core/RecordTable Object Reference"))
  (bind _returnvalue (`GameplayStatics.LoadGameFromSlot` (`self.RecordTableName`)))
  (`/Engine/EditorBlueprintResources/StandardMacros.IsValid` _returnvalue
    (:`Is Valid`
      (bind _asrecord_table (cast `/Game/Core/RecordTable` _returnvalue)
        (:`then`
          (set `local.Table` _asrecord_table))
        (:`CastFailed`
          (bind _returnvalue_2 (`GameplayStatics.CreateSaveGameObject` "/Game/Core/RecordTable.RecordTable_C" :!label _label))
          (bind _output_get (set `local.Table` _returnvalue_2)))))
    (:`Is Not Valid`
      (goto _label)))
  (return _output_get))