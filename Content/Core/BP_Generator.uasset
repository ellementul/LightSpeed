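; BP_Generator is a procedural block spawner that registers with BP_GI and steadily raises its Hard difficulty value over time.
; Run rolls each seed pattern's chance plus Hard, spawning its blocks on success, and each pattern's Continue rule decides whether evaluation proceeds.
; Blocks spawn relative to the calling Owner's generator transform at 90% scale for collision checks, then return to full scale and receive a generator reference.
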(event `self.ReceiveBeginPlay`
  (bind _asbp_gi (cast `/Game/Core/BP_GI` (`GameplayStatics.GetGameInstance`)))
  (set `/Game/Core/BP_GI.Generator` self _asbp_gi))

(event `self.ReceiveTick`
  (params (DeltaSeconds :type "Float (single-precision)"))
  (set `self.Hard` (+ (* DeltaSeconds (`self.HardAccel`)) (`self.Hard`))))

(fn `CheckPattern`
  (params (BlockPattern :type "/Game/Blocks/Core/BlockPattern Structure (by ref)"))
  (returns (IsContinue :type Boolean) (ReturnState :type "/Game/Blocks/Core/ConditionVariants Enum"))
  (locals (State :type "/Game/Blocks/Core/ConditionVariants Enum"))
  (bind (_blocks _change _continue) (break `/Game/Blocks/Core/BlockPattern` BlockPattern))
  (bind _state (`local.State`))
  (set `self.IsContinue` (`|EnumEquality` _continue "NewEnumerator3"))
  (`/Engine/EditorBlueprintResources/StandardMacros.CompareFloat` _change 1.0
    (:`>`
      (set `local.State` "NewEnumerator1" :!label _label))
    (:`==`
      (goto _label))
    (:`<`
      (`/Engine/EditorBlueprintResources/StandardMacros.CompareFloat` (+ _change (`self.Hard`)) (`KismetMathLibrary.RandomFloatInRange` 0.0 1.0)
        (:`>`
          (goto _label))
        (:`==`
          (goto _label))
        (:`<`
          (set `local.State` "NewEnumerator2")))))
  (return (or (`|EnumEquality` _state _continue) (`self.IsContinue`)) _state))

(fn `GeneratePattern`
  (params (Array :type "Array of /Game/Blocks/Core/Block Structure") (Owner :type "/Game/Blocks/Core/BaseBlock Object Reference"))
  (for _array_element Array
    (bind (_block _relativelocation _rotate) (break `/Game/Blocks/Core/Block` _array_element))
    (`self.SpawnBlock` _block Owner _relativelocation _rotate))
  (return))

(fn `Run`
  (params (Seed :type "/Game/Blocks/Core/Seed Structure (by ref)") (Owner :type "/Game/Blocks/Core/BaseBlock Object Reference"))
  (for _array_element (`.Patterns_3_0967AFF3454C4F6244D8A18E7BBE7029` (break `/Game/Blocks/Core/Seed` Seed))
    (bind (_iscontinue _returnstate) (`self.CheckPattern` _array_element))
    (if (`|EnumEquality` _returnstate "NewEnumerator1")
      (`self.GeneratePattern` (`.Blocks_3_0967AFF3454C4F6244D8A18E7BBE7029` (break `/Game/Blocks/Core/BlockPattern` _array_element)) Owner))
    (if (not _iscontinue)
      (break)))
  (return))

(fn `SpawnBlock`
  (params (Class :type "Actor Class Reference") (Owner :type "/Game/Blocks/Core/BaseBlock Object Reference") (RelLocation :type "Vector Structure") (RelRotate :type "Rotator Structure"))
  (bind (_dist_location _dist_rotation _dist_scale) (`KismetMathLibrary.BreakTransform` (`/Game/Blocks/Core/BaseBlock.GetGeneratorTramsform` Owner RelLocation)))
  (bind _returnvalue (`|SpawnActorFromClass` Class (`KismetMathLibrary.MakeTransform` _dist_location (`KismetMathLibrary.ComposeRotators` _dist_rotation RelRotate) (* _dist_scale (`KismetMathLibrary.MakeVector` 0.9 0.9 0.9))) "AdjustIfPossibleButDontSpawnIfColliding" "OverrideRootScale" self null))
  (`/Engine/EditorBlueprintResources/StandardMacros.IsValid` _returnvalue
    (:`Is Valid`
      (bind _asbase_block (cast `/Game/Blocks/Core/BaseBlock` _returnvalue))
      (set `/Game/Blocks/Core/BaseBlock.Generator` self _asbase_block)
      (`self.SetActorScale3D` _returnvalue _dist_scale)
      (return))))

(fn `UserConstructionScript`)