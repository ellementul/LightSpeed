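; BP_PC is the player controller that handles menu, pause and game-over flow.
; On BeginPlay it caches the GameHUD and spawns a BP_Toner actor linked to the controlled BP_Character.
; Pause input and ToggleMenu share one FlipFlop that toggles the HUD menu, cursor, input mode and game pause.
; Death stops PlayerState ticking and shows the HUD submit screen in UI-only input, while Submit calls GameOver on BP_GI.
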(event `self.ReceiveBeginPlay`
  (bind _asgame_hud (cast `/Game/Core/GameHUD` (`self.GetHUD`)))
  (set `self.HUD` _asgame_hud)
  (bind _asbp_character (cast `/Game/Character/BP_Character` (`self.K2_GetPawn`)))
  (bind _returnvalue (`|SpawnActorFromClass` "/Game/Core/BP_Toner.BP_Toner_C" (`KismetMathLibrary.MakeTransform` (0.0 0.0 0.0)) "AlwaysSpawn" "OverrideRootScale" null _asbp_character null))
  (set `self.Toner` _returnvalue))

(event `self.ReceiveTick`
  (params (DeltaSeconds :type "Float (single-precision)")))

(event `InputAction|Pause` :paused true
  (params (Key :type "Key Structure"))
  (bind _hud (`self.HUD`))
  (:`Pressed`
    (`/Engine/EditorBlueprintResources/StandardMacros.FlipFlop` :!label _label
      (:`A`
        (bind _widget (`/Game/Core/GameHUD.ShowMenu` _hud))
        (set `self.bShowMouseCursor` true)
        (`WidgetBlueprintLibrary.SetInputMode_GameAndUIEx` self _widget "DoNotLock" false)
        (`GameplayStatics.SetGamePaused` true))
      (:`B`
        (`/Game/Core/GameHUD.HideMenu` _hud)
        (set `self.bShowMouseCursor` false)
        (`WidgetBlueprintLibrary.SetInputMode_GameOnly` self)
        (`GameplayStatics.SetGamePaused` false)))))

(event `ToggleMenu`
  (goto _label))

(event `Death`
  (`self.SetActorTickEnabled` (`self.PlayerState`) false)
  (bind _widget (`/Game/Core/GameHUD.ShowSubmit` (`self.HUD`)))
  (set `self.bShowMouseCursor` true)
  (`WidgetBlueprintLibrary.SetInputMode_UIOnlyEx` self _widget))

(event `Submit`
  (bind _asbp_gi (cast `/Game/Core/BP_GI` (`GameplayStatics.GetGameInstance`)))
  (`/Game/Core/BP_GI.GameOver` _asbp_gi self))

(fn `UserConstructionScript`)